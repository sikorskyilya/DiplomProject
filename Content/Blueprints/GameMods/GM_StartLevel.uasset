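; Game mode for the start level that acts as a lobby, tracking player controllers and matchmaking queued players onto game servers.
; BeginPlay loads shop items and the server list from data tables, then starts looping timers to refresh controllers, run matchmaking and advance busy servers' game clocks.
; The matchmaker selects an idle "Game" server, calls Open on queued players, and marks it busy when full or its countdown expires, then seeks another.
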(event Custom|Matchmaker
  (bind _playersqueu (Variables|Default|GetPlayersQueu))
  (if (and (> (Utilities|Array|Length (Variables|Default|GetPlayersQueu)) 0) (Utilities|Enum|NotEqual(Enum) (.ipadress (Variables|Default|GetCurrentServer)) ""))
    (if (== (.serverstatus (Variables|Default|GetCurrentServer)) 0)
      (Variables|Default|SetCurrentServer (Utilities|Struct|MakeGameIpAdrr (.ipadress (Variables|Default|GetCurrentServer)) (.type (Variables|Default|GetCurrentServer)) (.countofplayers (Variables|Default|GetCurrentServer)) (.currentcountofplayers (Variables|Default|GetCurrentServer)) 1 0))
      (bind _result (Math|Integer|IncrementInt (Variables|Default|GetServerTime))
        (:%20%20
          _)))
    (if (== (.serverstatus (Variables|Default|GetCurrentServer)) 1)
      (if (>= (Variables|Default|GetServerTime) 29)
        (bind _output_get (Variables|Default|SetCurrentServer (Utilities|Struct|MakeGameIpAdrr (.ipadress (Variables|Default|GetCurrentServer)) (.type (Variables|Default|GetCurrentServer)) (.countofplayers (Variables|Default|GetCurrentServer)) (.currentcountofplayers (Variables|Default|GetCurrentServer)) 2 0)))
        (for (_array_element _array_index) (Variables|Default|GetServers)
          (if (Utilities|Enum|Equal(Enum) (.ipadress _array_element) (.ipadress (Variables|Default|GetCurrentServer)))
            (Utilities|Array|SetArrayElem (Variables|Default|GetServers) _array_index (Variables|Default|GetCurrentServer))))
        (CallFunction|ReadyServerIsExist)
        (else
          (for _array_element_2 _playersqueu
            (bind _isfull (CallFunction|UpdateServerInfoPlayers))
            (if _isfull
              (Variables|Default|SetCurrentServer (Utilities|Struct|MakeGameIpAdrr (.ipadress (Variables|Default|GetCurrentServer)) (.type (Variables|Default|GetCurrentServer)) (.countofplayers (Variables|Default|GetCurrentServer)) (.currentcountofplayers (Variables|Default|GetCurrentServer)) 2 0))
              (for (_array_element_3 _array_index_2) (Variables|Default|GetServers)
                (if (Utilities|Enum|Equal(Enum) (.ipadress _array_element_3) (.ipadress (Variables|Default|GetCurrentServer)))
                  (Utilities|Array|SetArrayElem (Variables|Default|GetServers) _array_index_2 (Variables|Default|GetCurrentServer))))
              (CallFunction|ReadyServerIsExist)
              (else
                (Default|Open _array_element_2)
                (Utilities|Array|RemoveItem _playersqueu _array_element_2))))))
      (else
        (CallFunction|ReadyServerIsExist)))
    (elif (== (.serverstatus (Variables|Default|GetCurrentServer)) 1)
      (bind _result_2 (Math|Integer|IncrementInt (Variables|Default|GetServerTime))
        (:%20%20
          (if (>= (Variables|Default|GetServerTime) 29)
            (bind _output_get_2 (Variables|Default|SetCurrentServer (Utilities|Struct|MakeGameIpAdrr (.ipadress (Variables|Default|GetCurrentServer)) (.type (Variables|Default|GetCurrentServer)) (.countofplayers (Variables|Default|GetCurrentServer)) (.currentcountofplayers (Variables|Default|GetCurrentServer)) 2 0)))
            (for (_array_element_4 _array_index_3) (Variables|Default|GetServers)
              (if (Utilities|Enum|Equal(Enum) (.ipadress _array_element_4) (.ipadress (Variables|Default|GetCurrentServer)))
                (Utilities|Array|SetArrayElem (Variables|Default|GetServers) _array_index_3 (Variables|Default|GetCurrentServer))))
            (CallFunction|ReadyServerIsExist)))))))

(event Custom|CheckGameServers
  ;[1 1 1] Mtch
  (CallFunction|CheckServers))

(event Custom|TimerFunction
  ;[1 1 1] Mtch
  (CallFunction|Matchmaker))

(event Custom|Refresh%20values
  (for _array_element (Variables|Default|GetPlayersControllers)
    (bind _aspc_start_level (Utilities|Casting|CastToPC_StartLevel _array_element))
    (Default|RefreshValues _aspc_start_level)))

(event Custom|GM_ShopData
  (CallFunction|SetUserShop))

(event Custom|Check%20servers
  (bind _servers (Variables|Default|GetServers))
  (for (_array_element _array_index) (Variables|Default|GetServers)
    (if (== (.serverstatus _array_element) 2)
      (if (not (>= (.currentservergametime _array_element) 150))
        (Utilities|Array|SetArrayElem _servers _array_index (Utilities|Struct|MakeGameIpAdrr (.ipadress (Utilities|Array|Get(acopy) _servers _array_index)) (.type (Utilities|Array|Get(acopy) _servers _array_index)) (.countofplayers (Utilities|Array|Get(acopy) _servers _array_index)) (.currentcountofplayers (Utilities|Array|Get(acopy) _servers _array_index)) (.serverstatus (Utilities|Array|Get(acopy) _servers _array_index)) (+ (.currentservergametime (Utilities|Array|Get(acopy) _servers _array_index)) 3)))))))

(event Custom|GM_ServerShopData
  (CallFunction|SetUserShop))

(event Custom|SetUserShop)

(event Custom|add
  (CallFunction|GMServerShopData))

(event EventOnLogout
  (params (ExitingController :type Controller%20Object%20Reference))
  (bind _aspc_start_level (Utilities|Casting|CastToPC_StartLevel ExitingController))
  (Utilities|Array|RemoveItem (Variables|Default|GetPlayersControllers) _aspc_start_level))

(event EventBeginPlay
  (Utilities|FlowControl|Delay 1.0)
  (bind _outrownames (DataTable|GetDataTableRowNames "/Game/Blueprints/DataTables/DT_CharacterModels.DT_CharacterModels"))
  (for _array_element _outrownames
    (bind _returnvalue (Utilities|GetDataTableRow "/Game/Blueprints/DataTables/DT_CharacterModels.DT_CharacterModels" _array_element)
      (:then
        (Utilities|Array|AddUnique (Variables|Default|GetShopGameObjects) _returnvalue)
        (for _array_element_2 (Variables|Default|GetPlayersControllers)
          (bind _aspc_start_level (Utilities|Casting|CastToPC_StartLevel _array_element_2))
          (Default|RefreshValues _aspc_start_level)))))
  (Utilities|Time|SetTimerbyEvent (delegate Custom|Refresh%20values) 1.5 true)
  (bind _outrownames_2 (DataTable|GetDataTableRowNames "/Game/Blueprints/DataTables/DT_ServerAdress.DT_ServerAdress"))
  (for _array_element_3 _outrownames_2
    (bind _returnvalue_2 (Utilities|GetDataTableRow "/Game/Blueprints/DataTables/DT_ServerAdress.DT_ServerAdress" _array_element_3)
      (:then
        (Utilities|Array|AddUnique (Variables|Default|GetServers) _returnvalue_2))))
  ;[1 1 1] Mtch
  (CallFunction|ReadyServerIsExist)
  (Utilities|Time|SetTimerbyEvent (delegate Custom|TimerFunction) 1.0 true)
  (Utilities|Time|SetTimerbyEvent (delegate Custom|CheckGameServers) 3.0 true))

(event EventPostLogin
  (params (NewPlayer :type Player%20Controller%20Object%20Reference))
  (bind _aspc_start_level (Utilities|Casting|CastToPC_StartLevel NewPlayer))
  (Default|Login _aspc_start_level)
  (Utilities|Array|AddUnique (Variables|Default|GetPlayersControllers) NewPlayer))

(fn ConstructionScript)

(fn ReadyServerIsExist
  (for _array_element (Variables|Default|GetServers)
    (if (and (Utilities|Enum|Equal(Enum) (.type _array_element) "Game") (== (.serverstatus _array_element) 0))
      (Variables|Default|SetCurrentServer (Utilities|Struct|MakeGameIpAdrr (.ipadress _array_element) (.type _array_element) (.countofplayers _array_element) (.currentcountofplayers _array_element) (.serverstatus _array_element) 0))
      (Variables|Default|SetServerTime 0)
      (return)))
  (return))

(fn UpdateServerInfoPlayers
  (if (Utilities|Enum|NotEqual(Enum) (.ipadress (Variables|Default|GetCurrentServer)) "")
    (for _array_element (Variables|Default|GetServers)
      (if (Utilities|Enum|Equal(Enum) (.ipadress _array_element) (.ipadress (Variables|Default|GetCurrentServer)))
        (if (< (.currentcountofplayers _array_element) (.countofplayers _array_element))
          (Math|Integer|IncrementInt (.countofplayers _array_element)
            (:%20%20
              (return false)))
          (else
            (return true)))))))

(fn ServerTimer
  (if (Variables|Default|GetEnableServer?)
    (if (>= (Variables|Default|GetServerTime) 29)
      (CallFunction|ReadyServerIsExist)
      (else
        (bind _result (Math|Integer|IncrementInt (Variables|Default|GetServerTime)))))))