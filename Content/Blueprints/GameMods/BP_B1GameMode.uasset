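; Game mode that runs timed matchmaking, starting a match after a fixed delay from the first player login.
; When the timer fires, it calls MatchCreation, destroys spectator pawns and calls ResetPlayers.
; It then sets each character's mesh from the DT_CharacterModels row matching its controller's one-based Index and shows in-progress widgets.
; A delegate bound at BeginPlay relays match state changes to those controllers' widgets.
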(event Custom|CustomEvent_0
  (Class|B1GameMode|MatchCreation)
  (bind _outactors (Actor|GetAllActorsOfClass "/Script/Engine.SpectatorPawn"))
  (for _array_element _outactors
    (Actor|DestroyActor _array_element))
  (Class|B1GameMode|ResetPlayers)
  (bind _outactors_2 (Actor|GetAllActorsOfClass "/Game/MainPCharacter.MainPCharacter_C"))
  (for _array_element_2 _outactors_2
    (bind _asbp_main_player_controller (Utilities|Casting|CastToBP_MainPlayerController (Pawn|GetController _array_element_2)))
    (bind _outrownames (DataTable|GetDataTableRowNames "/Game/Blueprints/DataTables/DT_CharacterModels.DT_CharacterModels"))
    (for (_array_element_3 _array_index) _outrownames
      (bind _returnvalue (Utilities|GetDataTableRow "/Game/Blueprints/DataTables/DT_CharacterModels.DT_CharacterModels" _array_element_3)
        (:then
          (if (== (+ _array_index 1) (Variables|/Game/Blueprints/Player/BP_MainPlayerController.BP_MainPlayerController_C|GetIndex _asbp_main_player_controller))
            (Class|SkinnedMeshComponent|SetSkeletalMesh (Variables|/Script/Engine.Character|GetMesh _array_element_2) (.charactermodel _returnvalue) true)
            (Default|ShowWidgets _asbp_main_player_controller "InProgress")))))))

(event Custom|OnTestDelegate_Event_0
  (params (MatchState :type EMatchState%20Enum :default "WaitingToStart"))
  (bind _outactors (Actor|GetAllActorsOfClass "/Game/MainPCharacter.MainPCharacter_C"))
  (for _array_element _outactors
    (bind _asbp_main_player_controller (Utilities|Casting|CastToBP_MainPlayerController (Pawn|GetController _array_element)))
    (Default|ShowWidgets _asbp_main_player_controller MatchState)))

(event EventBeginPlay
  (EventDispatchers|AssignOnTestDelegate (delegate Custom|OnTestDelegate_Event_0)))

(event EventFunqwe
  (Development|PrintString "Hello"))

(event EventPostLogin
  (params (NewPlayer :type Player%20Controller%20Object%20Reference))
  (if (not (Variables|Default|GetWasStarted))
    (Variables|Default|SetWasStarted true)
    ;[1 1 1] Matchmaker
    (Utilities|Time|SetTimerbyEvent (delegate Custom|CustomEvent_0) 3e+01)
    (Utilities|Array|Add (Variables|Default|GetPlayers) NewPlayer)))

(fn ConstructionScript)