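; Player controller that puts up the player's UI according to the state of the match.
; On BeginPlay it copies the user's character index from B1GameInst into its own Index variable.
; ShowWidgets switches on the matching state, creating the main player widget when play is in progress, or clearing all widgets and showing the game-over screen when it ends.
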(event Custom|ShowWidgets
  (params (MatchingState :type EMatchState%20Enum :default "WaitingToStart"))
  (bind _self self)
  (switch Utilities|FlowControl|Switch|SwitchonEMatchState MatchingState
    (:InProgress
      (bind _returnvalue (UserInterface|CreateWidget "/Game/Blueprints/Widgets/UI/W_MainPlayer.W_MainPlayer_C" _self))
      (UserInterface|Viewport|AddtoViewport _returnvalue 0))
    (:GameOver
      (Viewport|RemoveAllWidgets)
      (bind _returnvalue_2 (UserInterface|CreateWidget "/Game/Blueprints/Widgets/UI/W_GameOverBP.W_GameOverBP_C" _self))
      (UserInterface|Viewport|AddtoViewport _returnvalue_2 0))))

(event EventBeginPlay
  (bind _asb1game_inst (Utilities|Casting|CastToB1GameInst (Game|GetGameInstance)))
  (Variables|Default|SetIndex (Variables|/Game/B1GameInst.B1GameInst_C|GetUserCharacterIndex _asb1game_inst)))

(event EventTick
  (params (DeltaSeconds :type Float%20%28single-precision%29)))

(fn ConstructionScript)