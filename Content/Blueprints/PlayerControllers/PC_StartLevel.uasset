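; Player controller for the start level that handles account login, nickname setup, stat refresh, item purchases and match queueing.
; VaRest GET calls hit PHP scripts, usually with hard-coded-key encrypted credentials; nickname requests send them plain.
; Callbacks store status and player stats in B1GameInst and show the nickname form for new accounts; the purchase callback is empty.
; It also queues itself in GM_StartLevel and triggers CallShopItem when GameCharacterModels replicates.
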(event Custom|login
  (bind _returnvalue (Class|KismetSystemLibrary|GetDeviceId))
  ;[1 1 1] Client login
  (if (Utilities|Enum|Equal(Enum) _returnvalue "")
    (CallFunction|LoginServer "123" "il" "qw")
    (else
      (bind _asb1game_inst (Utilities|Casting|CastToB1GameInst (Game|GetGameInstance)))
      (bind _returnvalue_2 (Class|ServicesBF|Encrypt (Utilities|String|ToString(Text) (Variables|/Game/B1GameInst.B1GameInst_C|GetLogin _asb1game_inst)) "IlyaSikorsky"))
      (bind _returnvalue_3 (Class|ServicesBF|Encrypt (Utilities|String|ToString(Text) (Variables|/Game/B1GameInst.B1GameInst_C|GetPass _asb1game_inst)) "IlyaSikorsky"))
      (CallFunction|LoginServer _returnvalue _returnvalue_2 _returnvalue_3))))

(event Custom|Disable%20Interface
  (Class|PlayerController|ActivateTouchInterface (Game|GetPlayerController 0)))

(event Custom|SetRefreshValues
  (params (Silver :type String) (Gold :type String) (Rating :type String) (UserKills :type String) (UserBattles :type String) (Death :type String) (Nick :type String))
  (bind _asb1game_inst (Utilities|Casting|CastToB1GameInst (Game|GetGameInstance)))
  (Variables|/Game/B1GameInst.B1GameInst_C|SetUserGold _asb1game_inst (Math|Conversions|ToInteger(Byte) Gold))
  (Variables|/Game/B1GameInst.B1GameInst_C|SetUserSilver _asb1game_inst (Math|Conversions|ToInteger(Byte) Silver))
  (Variables|/Game/B1GameInst.B1GameInst_C|SetUserRating _asb1game_inst (Math|Conversions|ToInteger(Byte) Rating))
  (Variables|/Game/B1GameInst.B1GameInst_C|SetUserKills _asb1game_inst (Math|Conversions|ToInteger(Byte) UserKills))
  (Variables|/Game/B1GameInst.B1GameInst_C|SetUserBattles _asb1game_inst (Math|Conversions|ToInteger(Byte) UserBattles))
  (Variables|/Game/B1GameInst.B1GameInst_C|SetUserDeath _asb1game_inst (Math|Conversions|ToInteger(Byte) Death))
  (Variables|/Game/B1GameInst.B1GameInst_C|SetUserName _asb1game_inst Nick))

(event Custom|CustomEvent_3
  (params (Request :type Va%20Rest%20Request%20JSON%20Object%20Reference))
  (CallFunction|SetStatus (Variables|/Script/VaRest.VaRestRequestJSON|GetResponseContent Request)))

(event Custom|Open)

(event Custom|ShopData
  (CallFunction|Client (Variables|Default|GetGameCharacterModels)))

(event Custom|Shop]
  (CallFunction|ShopData))

(event Custom|Client
  (params (GameShop :type Array%20of%20Game%20Character%20Models%20Structures))
  (Variables|Default|SetGameCharacterModels GameShop))

(event Custom|BuyItem
  (params (ItemName :type Text) (Login :type Text) (Pass :type Text) (Sil :type Integer) (Gold :type Integer))
  ;[1 1 1] Buy Item
  (CallFunction|BuyItemonServer ItemName Login Pass Sil Gold))

(event Custom|BuyItemOnServer
  (params (Item :type Text) (Login :type Text) (Pass :type Text) (Silver :type Integer) (Gold :type Integer))
  (bind _returnvalue (|VaRestSubsystem))
  ;[1 1 1] Buy Item
  (bind _returnvalue_2 (Class|VaRestSubsystem|ConstructVaRestJsonObject _returnvalue))
  (bind _returnvalue_3 (Class|ServicesBF|Encrypt (Utilities|String|ToString(Text) Login) "IlyaSikorsky"))
  (bind _returnvalue_4 (Class|ServicesBF|Encrypt (Utilities|String|ToString(Text) Pass) "IlyaSikorsky"))
  (Class|VaRestSubsystem|CallURL _returnvalue (Utilities|String|Append "http://gunsfestival.mygamesonline.org/BuyItem.php?Login=" _returnvalue_3 "&Pass=" _returnvalue_4 "&Sil=" (Utilities|String|ToString(Integer) Silver) "&Gold=" (Utilities|String|ToString(Integer) Gold)) "GET" "x_www_form_urlencoded_url" _returnvalue_2 (delegate Custom|CustomEvent_2)))

(event Custom|CustomEvent_1
  (params (Request :type Va%20Rest%20Request%20JSON%20Object%20Reference))
  (bind _output_get (Variables|Default|SetResourseArray (Utilities|String|ParseIntoArray (Variables|/Script/VaRest.VaRestRequestJSON|GetResponseContent Request) " ")))
  (CallFunction|SetRefreshValues (.RightS (Utilities|String|Split (Utilities|Array|Get(acopy) _output_get 3) "=")) (.RightS (Utilities|String|Split (Utilities|Array|Get(acopy) _output_get 4) "=")) (.RightS (Utilities|String|Split (Utilities|Array|Get(acopy) _output_get 2) "=")) (.RightS (Utilities|String|Split (Utilities|Array|Get(acopy) _output_get 1) "=")) (.RightS (Utilities|String|Split (Utilities|Array|Get(acopy) _output_get) "=")) (.RightS (Utilities|String|Split (Utilities|Array|Get(acopy) _output_get 5) "=")) (.RightS (Utilities|String|Split (Utilities|Array|Get(acopy) _output_get 6) "="))))

(event Custom|Check%20nickname
  (params (NickName :type Text))
  (bind _asb1game_inst (Utilities|Casting|CastToB1GameInst (Game|GetGameInstance)))
  (CallFunction|NickNameonServer NickName (Variables|/Game/B1GameInst.B1GameInst_C|GetLogin _asb1game_inst) (Variables|/Game/B1GameInst.B1GameInst_C|GetPass _asb1game_inst)))

(event Custom|login%20server
  (params (Id :type String) (Login :type String) (Password :type String))
  (bind _returnvalue (|VaRestSubsystem))
  ;[1 1 1] Login request
  (bind _returnvalue_2 (Class|VaRestSubsystem|ConstructVaRestJsonObject _returnvalue))
  (Class|VaRestSubsystem|CallURL _returnvalue (Utilities|String|Append "http://gunsfestival.mygamesonline.org/LoginRegistration.php?ID=" Id "&Login=" Login "&Pass=" Password) "GET" "x_www_form_urlencoded_url" _returnvalue_2 (delegate Custom|CustomEvent)))

(event Custom|NickNameOnServer
  (params (NickName :type Text) (Login :type Text) (Pass :type Text))
  (bind _returnvalue (|VaRestSubsystem))
  (bind _returnvalue_2 (Class|VaRestSubsystem|ConstructVaRestJsonObject _returnvalue))
  (Class|VaRestSubsystem|CallURL _returnvalue (Utilities|String|Append "http://gunsfestival.mygamesonline.org/Nickname.php?Nick=" (Utilities|String|ToString(Text) NickName) "&Login=" (Utilities|String|ToString(Text) Login) "&Pass=" (Utilities|String|ToString(Text) Pass)) "GET" "x_www_form_urlencoded_url" _returnvalue_2 (delegate Custom|CustomEvent_3)))

(event Custom|CustomEvent
  (params (Request :type Va%20Rest%20Request%20JSON%20Object%20Reference))
  ;[1 1 1] Login request
  (CallFunction|LoginandSaveStatus (Variables|/Script/VaRest.VaRestRequestJSON|GetResponseContent Request) (Utilities|Text|ToText(String) (stale Custom|login%20server Login)) (Utilities|Text|ToText(String) (stale Custom|login%20server Password))))

(event Custom|SetStatus
  (params (Status :type String))
  (Variables|Default|SetNickStatus Status))

(event Custom|CustomEvent_2
  (params (Request :type Va%20Rest%20Request%20JSON%20Object%20Reference))
  ;[1 1 1] Buy Item
)

(event Custom|Game
  (bind _asgm_start_level (Utilities|Casting|CastToGM_StartLevel (Game|GetGameMode)))
  (Utilities|Array|AddUnique (Variables|/Game/Blueprints/GameMods/GM_StartLevel.GM_StartLevel_C|GetPlayersQueu _asgm_start_level) self))

(event Custom|LoginAndSaveStatus
  (params (Status :type String) (Login :type Text) (Pass :type Text) (Nick :type String))
  (bind _asb1game_inst (Utilities|Casting|CastToB1GameInst (Game|GetGameInstance)))
  (bind _output_get (Variables|/Game/B1GameInst.B1GameInst_C|SetStatus _asb1game_inst Status))
  (Variables|/Game/B1GameInst.B1GameInst_C|SetUserName _asb1game_inst "")
  (if (Utilities|Enum|Equal(Enum) _output_get "New")
    (Viewport|RemoveAllWidgets)
    (bind _returnvalue (UserInterface|CreateWidget "/Game/Blueprints/Widgets/W_NickNameForm.W_NickNameForm_C"))
    (UserInterface|Viewport|AddtoViewport _returnvalue 0)))

(event Custom|Response
  (params (Request :type Va%20Rest%20Request%20JSON%20Object%20Reference))
  (if (Utilities|Enum|Equal(Enum) "Ok" (Variables|/Script/VaRest.VaRestRequestJSON|GetResponseContent Request))
    _))

(event Custom|Add%20to%20queu
  (CallFunction|Game))

(event Custom|RefreshValues
  (bind _asb1game_inst (Utilities|Casting|CastToB1GameInst (Game|GetGameInstance)))
  (bind _returnvalue (Class|ServicesBF|Encrypt (Utilities|String|ToString(Text) (Variables|/Game/B1GameInst.B1GameInst_C|GetLogin _asb1game_inst)) "IlyaSikorsky"))
  (bind _returnvalue_2 (Class|ServicesBF|Encrypt (Utilities|String|ToString(Text) (Variables|/Game/B1GameInst.B1GameInst_C|GetPass _asb1game_inst)) "IlyaSikorsky"))
  (CallFunction|RefreshValuesServer _returnvalue _returnvalue_2))

(event Custom|RefreshValuesServer
  (params (UserLogin :type String) (UserPass :type String))
  (bind _returnvalue (|VaRestSubsystem))
  (bind _returnvalue_2 (Class|VaRestSubsystem|ConstructVaRestJsonObject _returnvalue))
  (Class|VaRestSubsystem|CallURL _returnvalue (Utilities|String|Append "http://gunsfestival.mygamesonline.org/GetUserValues.php?Login=" UserLogin "&Pass=" UserPass) "GET" "x_www_form_urlencoded_url" _returnvalue_2 (delegate Custom|CustomEvent_1)))

(event EventBeginPlay
  (Variables|Default|SetbShowMouseCursor true)
  (CallFunction|DisableInterface))

(fn ConstructionScript)

(fn OnRepNewVar0)

(fn OnRepGameCharacterModels
  (Default|CallShopItem))